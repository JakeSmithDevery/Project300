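; BP_TestPlayer is a test player Blueprint for exercising the quest and enemy-death systems.
; BeginPlay calls the parent logic, then starts Quest1 through its Quest reference.
; A debug key handler on K release casts to BP_GameMode and records a death for Enemy01, simulating a kill.
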(event EventBeginPlay
  (|CallParentFunction)
  (Class|QuestComponent|StartQuest (Variables|Default|GetQuest) "/Game/Peter/Quest/Quest1/Quest1.Quest1"))

(event Collision|EventActorBeginOverlap
  (params (OtherActor :type Actor%20Object%20Reference)))

(event EventTick
  (params (DeltaSeconds :type Float%20%28single-precision%29))
  (|CallParentFunction DeltaSeconds) ; This node is disabled and will not be called.\nDrag off pins to build functionality.
)

(event Input|KeyboardEvents|DebugKeyK
  (params (Key :type Key%20Structure :default "None") (ActionValue :type Input%20Action%20Value%20Structure))
  (:Released
    (bind _asbp_game_mode (Utilities|Casting|CastToBP_GameMode (Game|GetGameMode)))
    (Class|CustomGameMode|RecordEnemyDeath _asbp_game_mode "Enemy01")))

(fn ConstructionScript
  (|CallParentFunction))