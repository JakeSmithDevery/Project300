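; BP_Game is a music manager that plays, stops, pauses and resumes a single active 2D music track.
; PlayMusic fades out any valid active player, then creates a 2D sound that persists across level transitions, stores it as active and fades it in.
; The two fade inputs are stored crosswise, so FadeInNewTime drives the old track's fade-out and FadeOutOldTime the new track's fade-in.
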(event `/Game/Robert/BPI_MusicPlayer.PlayMusic`
  (params (Music :type "SoundBase Object Reference") (FadeInNewTime :type "Float (double-precision)") (FadeOutOldTime :type "Float (double-precision)"))
  ;[0.2266 0.5885 0] Play
  ;;[1 1 1] Set Local Variables
  (set `self.Music` Music)
  (set `self.Fade Out Time Old` FadeInNewTime)
  (set `self.Fade in Time New` FadeOutOldTime)
  (`/Engine/EditorBlueprintResources/StandardMacros.IsValid` (`self.ActiveMusicPlayer`)
    (:`Is Valid`
      (`self.StopMusic` (`self.Fade Out Time Old`)))
    (:`Is Not Valid`
      _))
  ;;[1 0.1476 0.6953] FadeIn New
  (bind _returnvalue (`GameplayStatics.CreateSound2D` (`self.Music`) 1.0 1.0 0.0 null true))
  (bind _output_get (set `self.ActiveMusicPlayer` _returnvalue))
  (`AudioComponent.FadeIn` _output_get (`self.Fade in Time New`) 1.0 0.0 "Linear"))

(event `/Game/Robert/BPI_MusicPlayer.StopMusic`
  (params (FadeOutTime :type "Float (double-precision)"))
  ;[1 0 0] Stop
  (bind _output_get (set `self.FadeOutMusicPlayer` (`self.ActiveMusicPlayer`)))
  (`AudioComponent.FadeOut` _output_get FadeOutTime 0.0 "Linear"))

(event `/Game/Robert/BPI_MusicPlayer.PauseMusic`
  ;[1 0.6715 0] Pause
  (`AudioComponent.SetPaused` (`self.ActiveMusicPlayer`) true))

(event `/Game/Robert/BPI_MusicPlayer.ResumeMusic`
  ;[0.671 1 0] Resume
  (`AudioComponent.SetPaused` (`self.ActiveMusicPlayer`) false))