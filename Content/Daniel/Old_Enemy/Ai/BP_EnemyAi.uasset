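; Enemy pawn, stored under Old_Enemy, that spots the player and performs a forward melee-range attack.
; PawnSensing sets the "hasSeen?" Blackboard key when it sees BP_Player.
; AttackPlayer sphere-traces ahead for pawns, with debug drawing on, then plays a random montage on a hit player.
; It then calls ApplyDamage on that player with no damage amount set in the graph.
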(event `self.PawnSensing.OnSeePawn`
  (params (Pawn :type "Pawn Object Reference"))
  (cast `/Game/Jake/Character/Blueprints/BP_Player` Pawn)
  (`BlackboardComponent.SetValueAsBool` (`AIBlueprintHelperLibrary.GetBlackboard` (`AIBlueprintHelperLibrary.GetAIController` self)) "hasSeen?" true))

(event `AttackPlayer`
  (bind _returnvalue (`self.K2_GetActorLocation`))
  (bind _newvar_0 (`self.NewVar_0`))
  ;[1 1 1] this creates a sphere from enemies location and shoots it directly forward
  ; radius=size, End = How far the beam goes
  (bind (_outhit _returnvalue_2) (`KismetSystemLibrary.SphereTraceSingleForObjects` :`Start` _returnvalue :`End` (+ _returnvalue (* (`KismetMathLibrary.GetForwardVector` (`self.K2_GetActorRotation`)) 250.0)) :`Radius` 120.0 :`ObjectTypes` (`|MakeArray` "ObjectTypeQuery3" :!type "EObjectTypeQuery Enum") :`DrawDebugType` "ForDuration"))
  (if _returnvalue_2
    (bind (_bblockinghit _binitialoverlap _time _distance _location _impactpoint _normal _impactnormal _physmat _hitactor) (`GameplayStatics.BreakHitResult` _outhit))
    ;[1 1 1] checks if the player got hit
    (bind _asbp_player (cast `/Game/Jake/Character/Blueprints/BP_Player` _hitactor))
    (`self.PlayAnimMontage` _asbp_player (`|GetArrayItem` _newvar_0 (`KismetMathLibrary.RandomInteger` (`KismetArrayLibrary.Array_Length` _newvar_0))) 1.0 "None")
    (`GameplayStatics.ApplyDamage` _hitactor)))

(fn `UserConstructionScript`)