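; BP_EnemyBase is a base enemy character that exposes health, damage, patrol route, ideal ranges and movement speed to other systems.
; BPCDamageSystem handles damage and health queries, while Heal forwards to the HealthBar rather than the damage system.
; BeginPlay caches the AIC_EnemyBase controller, creates the health bar widget and binds the damage system's OnDeath.
; Death ragdolls the mesh, stops AI logic and sets the controller's dead state.
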(event `self.ReceiveBeginPlay`
  (bind _asaic_enemy_base (cast `/Game/Daniel/New_Enemy/AI/AIC_EnemyBase` (`AIBlueprintHelperLibrary.GetAIController` self)))
  (set `self.As AIC Enemy Base` _asaic_enemy_base)
  (bind _returnvalue (`|CreateWidget` "/Game/Daniel/New_Enemy/AI/DamageSystem/W_HealthBar.W_HealthBar_C" null self))
  (`WidgetComponent.SetWidget` (`self.HealthBar`) _returnvalue)
  (add `/Game/Daniel/New_Enemy/AI/DamageSystem/BPC_DamageSystem.OnDeath` (`self.BPC_DamageSystem`) (`|CreateDelegate` :!event `Death`)))

(event `Death`
  (bind _mesh (`self.Mesh`))
  (`PrimitiveComponent.SetSimulatePhysics` _mesh true)
  (`PrimitiveComponent.SetCollisionEnabled` _mesh "QueryAndPhysics")
  (`BrainComponent.StopLogic` (`AIController.BrainComponent` (`self.As AIC Enemy Base`)) "")
  (`/Game/Daniel/New_Enemy/AI/AIC_EnemyBase.SetStateAsDead` (`self.As AIC Enemy Base`)))

(fn `GetCurrentHealth`
  (returns (Health :type "Float (double-precision)"))
  (return (`/Game/Daniel/New_Enemy/AI/DamageSystem/BPC_DamageSystem.Health` (`self.BPC_DamageSystem`))))

(fn `GetIdealRange`
  (returns (AttackRadius :type "Float (double-precision)") (DefendRadius :type "Float (double-precision)"))
  (return 150.0 350.0))

(fn `GetMaxHealth`
  (returns (MaxHealth :type "Float (double-precision)"))
  (return (`/Game/Daniel/New_Enemy/AI/DamageSystem/BPC_DamageSystem.MaxHealth` (`self.BPC_DamageSystem`))))

(fn `GetPatrolRoute`
  (returns (PatrolRoute :type "/Game/Daniel/New_Enemy/AI/BP_PatrolRoute Object Reference"))
  (return (`self.PatrolRoute`)))

(fn `Heal`
  (params (Amount :type "Float (double-precision)"))
  (returns (NewHealth :type "Float (double-precision)"))
  (bind _newhealth (message `/Game/Daniel/New_Enemy/AI/DamageSystem/BPI_DamageSystem.Heal` (`self.HealthBar`) Amount))
  (return _newhealth))

(fn `IsDead`
  (returns (IsDead :type Boolean))
  (return (`/Game/Daniel/New_Enemy/AI/DamageSystem/BPC_DamageSystem.IsDead` (`self.BPC_DamageSystem`))))

(fn `SetMovementSpeed`
  (params (Speed :type "/Game/Daniel/New_Enemy/AI/Enums/E_MovementSpeed Enum" :default "NewEnumerator0"))
  (returns (SpeedValue :type "Float (double-precision)"))
  (bind _output_get (set `CharacterMovementComponent.MaxWalkSpeed` (select `/Game/Daniel/New_Enemy/AI/Enums/E_MovementSpeed` Speed :`NewEnumerator1` 100.0 :`NewEnumerator2` 300.0 :`NewEnumerator3` 500.0 :`NewEnumerator4` 200.0 :!type "Float (single-precision)") (`self.CharacterMovement`)))
  (return _output_get))

(fn `TakeDamage`
  (params (DamageInfo :type "/Game/Daniel/New_Enemy/AI/DamageSystem/S_DamageInfo Structure"))
  (returns (WasHit :type Boolean))
  (bind _washit (`/Game/Daniel/New_Enemy/AI/DamageSystem/BPC_DamageSystem.TakeDamage` (`self.BPC_DamageSystem`) DamageInfo))
  (return _washit))

(fn `UserConstructionScript`)