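; BP_SwordEnemy is a sword-wielding enemy that draws, swings and sheathes its weapon.
; Attack plays a montage and, on notify, sphere-traces forward for pawns to send damage through a TakeDamage message.
; WeildWeapon and UnWeildWeapon use unsheath and sheathe montage notifies to spawn and socket-attach the sword or destroy it, tracking the wielding flag.
; Dispatchers report when attack, wield and unwield montages finish.
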(event `/Game/Daniel/New_Enemy/AI/BPI_EnemyAI.Attack`
  (bind _returnvalue (`self.K2_GetActorLocation`))
  (bind _notifyname (`|PlayMontage` (`self.Mesh`) (`self.Anim Montage`))
    (:`OnCompleted`
      (`self.OnAttackEnd` :!label _label))
    (:`OnInterrupted`
      (goto _label))
    (:`OnNotifyBegin`
      (switch `name` _notifyname
        (:`Hit`
          (bind (_outhit _returnvalue_2) (`KismetSystemLibrary.SphereTraceSingleForObjects` :`Start` _returnvalue :`End` (+ _returnvalue (* (`self.GetActorForwardVector`) 200.0)) :`Radius` 50.0 :`ObjectTypes` (`|MakeArray` "ObjectTypeQuery3" :!type "EObjectTypeQuery Enum") :`DrawDebugType` "ForDuration"))
          (if _returnvalue_2
            (message `/Game/Daniel/New_Enemy/AI/DamageSystem/BPI_DamageSystem.TakeDamage` (`.HitActor` (`GameplayStatics.BreakHitResult` _outhit)) (make `/Game/Daniel/New_Enemy/AI/DamageSystem/S_DamageInfo` 25.0 "NewEnumerator1"))))))))

(event `/Game/Daniel/New_Enemy/AI/BPI_EnemyAI.WeildWeapon`
  ;[1 1 1] Spanws sword called at the start of aggresive state
  (if (not (`self.IsWieldingWeapon`))
    (bind _notifyname (`|PlayMontage` (`self.Mesh`) "/Game/Daniel/New_Enemy/Animation/Montage/AM_Unsheath.AM_Unsheath")
      (:`OnCompleted`
        (`self.OnWield`))
      (:`OnNotifyBegin`
        (switch `name` _notifyname
          (:`Unsheath`
            (`|SpawnActorFromClass` "/Game/Daniel/New_Enemy/Weapons/BPs/BP_Sword2.BP_Sword2_C" (`self.GetTransform`) "Undefined" "MultiplyWithRoot" null null)
            (bind _output_get (set `self.WeaponActor` null))
            (`self.K2_AttachToComponent` _output_get (`self.Mesh`) "hand_r_sword_socket" "SnapToTarget" "SnapToTarget" "SnapToTarget" true)
            (set `self.IsWieldingWeapon` true)
            (`self.WeildWeapon`)))))))

(event `/Game/Daniel/New_Enemy/AI/BPI_EnemyAI.UnWeildWeapon`
  ;[1 1 1] This is how actor is being despawned and sheath weapon is played
  (bind _notifyname (`|PlayMontage` (`self.Mesh`) "/Game/Daniel/New_Enemy/Animation/Montage/AM_Sheathing_Sword.AM_Sheathing_Sword")
    (:`OnCompleted`
      (`self.OnUnweild`))
    (:`OnNotifyBegin`
      (switch `name` _notifyname
        (:`PutAwaySword`
          (`self.K2_DestroyActor` (`self.WeaponActor`))
          (set `self.IsWieldingWeapon` false))))))

(fn `UserConstructionScript`
  (`parent.UserConstructionScript`))