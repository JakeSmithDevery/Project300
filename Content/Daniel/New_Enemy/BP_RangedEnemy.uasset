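; BP_RangedEnemy is a bow-wielding enemy that extends a parent enemy class with its own health and ideal attack and defend range.
; On BeginPlay it spawns BP_Bow and attaches it to the left-hand socket.
; Attack plays a bow-shot montage; its notify line-traces from bow to the AI controller's target, applying damage directly, without a projectile, when nothing blocks.
; Montage completion or interruption signals attack end.
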(event `self.ReceiveBeginPlay`
  (`parent.ReceiveBeginPlay`)
  (`self.WeildWeapon`))

(event `/Game/Daniel/New_Enemy/AI/BPI_EnemyAI.WeildWeapon`
  (bind _returnvalue (`|SpawnActorFromClass` "/Game/Daniel/New_Enemy/Weapons/BPs/BP_Bow.BP_Bow_C" (`KismetMathLibrary.MakeTransform` (0.0 0.0 0.0)) "Undefined" "MultiplyWithRoot" null null))
  (bind _output_get (set `self.WeaponActor` _returnvalue))
  (`self.K2_AttachToComponent` _output_get (`self.Mesh`) "hand_l_BowSocket" "SnapToTarget" "SnapToTarget" "SnapToTarget" true)
  (set `self.IsWieldingWeapon` true))

(event `/Game/Daniel/New_Enemy/AI/BPI_EnemyAI.Attack`
  (bind _notifyname (`|PlayMontage` (`self.Mesh`) "/Game/Daniel/New_Enemy/Animation/Montage/AM_BowShot.AM_BowShot")
    (:`OnCompleted`
      (`self.OnAttackEnd` :!label _label)
      (`KismetSystemLibrary.PrintString` "call attack shoot succesful"))
    (:`OnInterrupted`
      (goto _label))
    (:`OnNotifyBegin`
      (switch `name` _notifyname
        (:`Shot`
          (bind _asaic_enemy_base (cast `/Game/Daniel/New_Enemy/AI/AIC_EnemyBase` (`AIBlueprintHelperLibrary.GetAIController` self)))
          (bind _attack_target (`/Game/Daniel/New_Enemy/AI/AIC_EnemyBase.Attack Target` _asaic_enemy_base)
            (:`then`
              (bind (_outhit _returnvalue) (`KismetSystemLibrary.LineTraceSingle` :`Start` (`self.K2_GetActorLocation` (`self.WeaponActor`)) :`End` (`self.K2_GetActorLocation` _attack_target) :`TraceChannel` "TraceTypeQuery1" :`DrawDebugType` "ForDuration"))
              (if (not _returnvalue)
                (message `/Game/Daniel/New_Enemy/AI/DamageSystem/BPI_DamageSystem.TakeDamage` _attack_target (make `/Game/Daniel/New_Enemy/AI/DamageSystem/S_DamageInfo` 25.0 "NewEnumerator2"))))
            (:`else`
              (`KismetSystemLibrary.PrintString` "invalid"))))))))

(fn `GetIdealRange`
  (returns (AttackRadius :type "Float (double-precision)") (DefendRadius :type "Float (double-precision)"))
  (return 600.0 600.0))

(fn `UserConstructionScript`
  (bind _bpc_damagesystem (`self.BPC_DamageSystem`))
  (`parent.UserConstructionScript`)
  (set `/Game/Daniel/New_Enemy/AI/DamageSystem/BPC_DamageSystem.MaxHealth` 100.0 _bpc_damagesystem)
  (set `/Game/Daniel/New_Enemy/AI/DamageSystem/BPC_DamageSystem.Health` 100.0 _bpc_damagesystem))